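; BP_MasterGActor is a base actor for animated objects, offering helpers that move, rotate and scale a ToAnimate component.
; On BeginPlay it sets every Timeline component to a random time and a shared PlayRate, desynchronizing instances.
; Translate lerps relative location between the PosA and PosB markers by an alpha, while Rotate and Scale set relative rotation and scale directly.
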(event EventBeginPlay
  (for _array_element (Actor|GetComponentsByClass "/Script/Engine.TimelineComponent")
    (Components|Timeline|SetNewTime _array_element (Math|Random|RandomFloatinRange 0.0 (Components|Timeline|GetTimelineLength _array_element)))
    (Components|Timeline|SetPlayRate _array_element (Variables|Default|GetPlayRate))))

(fn ConstructionScript)

(fn Translate
  (params (Alpha :type Float%20%28double-precision%29))
  (Transformation|SetRelativeLocation (Variables|Default|Getto%20animate) (Math|Vector|Lerp(Vector) (Variables|/Script/Engine.SceneComponent|GetRelativeLocation (Variables|Default|GetPosA)) (Variables|/Script/Engine.SceneComponent|GetRelativeLocation (Variables|Default|GetPosB)) Alpha) false false)
  (return))

(fn Rotate
  (params (Roll :type Float%20%28double-precision%29) (Pitch :type Float%20%28double-precision%29) (Yaw :type Float%20%28double-precision%29))
  (Transformation|SetRelativeRotation (Variables|Default|Getto%20animate) (Math|Rotator|MakeRotator Roll Pitch Yaw) false false)
  (return))

(fn Scale
  (params (Scale :type Vector))
  (Transformation|SetRelativeScale3D (Variables|Default|Getto%20animate) Scale)
  (return))