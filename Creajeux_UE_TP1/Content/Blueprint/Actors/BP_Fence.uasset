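; BP_Fence is a fence actor that builds itself procedurally along an editable Spline component.
; The construction script adds a static mesh at each spline point, then a spline mesh between each pair of consecutive points.
; Each spline mesh takes the local locations and tangents of its two points, so the segments bend to follow the curve.
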(fn ConstructionScript
  (bind _spline (Variables|Default|GetSpline))
  (bind _spline_2 (Variables|Default|GetSpline))
  (for _index (range 0 (- (Spline|GetNumberOfSplinePoints _spline_2) 1))
    (AddComponent|AddStaticMeshComponent false (Math|Transform|MakeTransform (Spline|GetLocationatSplinePoint _spline_2 _index "Local") "0, 0, 0" "1.000000,1.000000,1.000000")))
  (for _index_2 (range 0 (- (Spline|GetNumberOfSplinePoints (Variables|Default|GetSpline)) 2))
    (bind _returnvalue (AddComponent|AddSplineMeshComponent false))
    (SplineMesh|SetStartandEnd _returnvalue (.Location (Spline|GetLocationandTangentatSplinePoint _spline _index_2 "Local")) (.Tangent (Spline|GetLocationandTangentatSplinePoint _spline _index_2 "Local")) (.Location (Spline|GetLocationandTangentatSplinePoint _spline (+ _index_2 1) "Local")) (.Tangent (Spline|GetLocationandTangentatSplinePoint _spline (+ _index_2 1) "Local")) true :!class /Script/Engine.SplineMeshComponent)))