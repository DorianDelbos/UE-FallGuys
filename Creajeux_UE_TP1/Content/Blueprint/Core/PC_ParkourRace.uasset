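; PC_ParkourRace is the player controller for a parkour race mode and handles the pause input.
; On BeginPlay it casts the current game mode to GM_ParkourRace and caches the reference.
; The IA_Pause Enhanced Input action toggles pause by passing the inverse of the current paused state to the game mode's SetPause, after checking that the Enhanced Input subsystem is valid.
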(event Input|EnhancedActionEvents|EnhancedInputActionIA_Pause
  (params (ActionValue :type Boolean) (ElapsedSeconds :type Float%20%28double-precision%29) (TriggeredSeconds :type Float%20%28double-precision%29) (InputAction :type Input%20Action%20Object%20Reference :default "/Game/Blueprint/Input/IA_Pause.IA_Pause"))
  ;[1 0.5 0] Pause
  (Utilities|IsValid (PlayerController|LocalPlayerSubsystems|GetEnhancedInputLocalPlayerSubsystem (Game|GetPlayerController 0))
    (:Is%20Valid
      (Default|SetPause (Variables|Default|GetGamemode) (not (Game|IsGamePaused))))))

(event EventBeginPlay
  ;[0.9556 0 1] Get Gamemode
  (bind _asgm_parkour_race (Utilities|Casting|CastToGM_ParkourRace (Game|GetGameMode)))
  (Variables|Default|SetGamemode _asgm_parkour_race))

(fn ConstructionScript)