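; BP_Checkpoint is a checkpoint prop that notifies the game mode through UpdateCheckpointMessage, passing itself, when its Box trigger is overlapped.
; The overlap does not filter which actor entered, and any further checkpoint handling is left to the game mode.
; The construction script gives the Plane a dynamic MI_Checkpoint material instance driven by the actor's SpeedX, SpeedY and Color variables.
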(event OnComponentBeginOverlap(Box)
  (params (OverlappedComponent :type Primitive%20Component%20Object%20Reference) (OtherActor :type Actor%20Object%20Reference) (OtherComp :type Primitive%20Component%20Object%20Reference) (OtherBodyIndex :type Integer) (bFromSweep :type Boolean) (SweepResult :type Hit%20Result%20Structure%20%28by%20ref%29))
  (Class|BPIPlayer|UpdateCheckpoint(Message) (Game|GetGameMode) self))

(fn ConstructionScript
  (bind _returnvalue (Rendering|Material|CreateDynamicMaterialInstance (Variables|Default|GetPlane) 0 "/Game/Material/MI_Checkpoint.MI_Checkpoint" "None" :!class /Script/Engine.PrimitiveComponent))
  (Rendering|Material|SetScalarParameterValue _returnvalue "SpeedX" (Variables|Default|GetSpeedX) :!class /Script/Engine.MaterialInstanceDynamic)
  (Rendering|Material|SetScalarParameterValue _returnvalue "SpeedY" (Variables|Default|GetSpeedY) :!class /Script/Engine.MaterialInstanceDynamic)
  (Rendering|Material|SetVectorParameterValue _returnvalue "Color" (Variables|Default|GetColor) :!class /Script/Engine.MaterialInstanceDynamic))