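; Temporary platform prop that scales away in a puff after being hit, then respawns.
; A hit on AnimatedMesh sets an Active guard and plays ScaleTimeLine, whose Alpha drives X and Y scale while Z stays fixed.
; When the timeline finishes, it spawns the NS_Poof effect, waits DelayBeforeRespawn, then clears the guard and restores full scale.
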(event OnComponentHit(AnimatedMesh)
  (params (HitComponent :type Primitive%20Component%20Object%20Reference) (OtherActor :type Actor%20Object%20Reference) (OtherComp :type Primitive%20Component%20Object%20Reference) (NormalImpulse :type Vector :default "0, 0, 0") (Hit :type Hit%20Result%20Structure%20%28by%20ref%29))
  (if (not (Variables|Default|GetActive))
    (Variables|Default|SetActive true)
    (bind _alpha (Timeline|ScaleTimeLine PlayFromStart)
      (:Update
        (CallFunction|Scale (Math|Vector|MakeVector _alpha _alpha 1.0)))
      (:Finished
        (Niagara|SpawnSystematLocation "/Game/ParkourRace/Assets/Niagara/NS_Poof.NS_Poof" (Transformation|GetActorLocation))
        (Utilities|FlowControl|Delay (Variables|Default|GetDelayBeforeRespawn))
        (Variables|Default|SetActive false)
        (CallFunction|Scale "1.000000,1.000000,1.000000")))))

(event EventBeginPlay
  (|CallParentFunction)
  (Components|Timeline|SetNewTime (Variables|Default|GetScaleTimeLine) 0.0))

(fn ConstructionScript
  (|CallParentFunction))