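; Game mode for a parkour race that handles checkpoints, respawning, pausing and the win transition.
; It stores the latest checkpoint and respawns by spawning and possessing a new P_MainChara at that checkpoint's arrow, falling back to a PlayerStart.
; Pausing updates the cached HUD and game pause state, then plays the pause animation.
; Winning plays the HUD match-over animation and opens the given level when it finishes.
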(event Custom|OnAnimFinish
  (CallFunction|OpenLevelName (stale EventWin Level)))

(event EventUpdateCheckpoint
  (params (NewCheckpoint :type BP%20Checkpoint%20Object%20Reference))
  (Variables|Default|SetCurrentCheckpoint NewCheckpoint))

(event EventWin
  (params (Level :type Name :default "None"))
  (bind _hudparkourrace (Variables|Default|GetHudParkourRace))
  (bind _hudui (Variables|/Game/Blueprint/Core/HUD_ParkourRace.HUD_ParkourRace_C|GetHudUi _hudparkourrace))
  (bind _matchoveranim (Variables|/Game/Blueprint/UI/W_HUDWidget.W_HUDWidget_C|GetMatchOverAnim _hudui))
  (Default|PlayAnim _hudui _matchoveranim 1.0)
  (Class|UserWidget|BindtoAnimationFinished _hudui _matchoveranim (delegate Custom|OnAnimFinish)))

(event EventBeginPlay
  (bind _ashud_parkour_race (Utilities|Casting|CastToHUD_ParkourRace (HUD|GetHUD (Game|GetPlayerController 0))))
  (Variables|Default|SetHudParkourRace _ashud_parkour_race))

(fn ConstructionScript)

(fn RespawnChara
  (Utilities|IsValid (Variables|Default|GetCurrentCheckpoint)
    (:Is%20Valid
      (LocalVariables|SetTransformToSpawn (Transformation|GetWorldTransform (Variables|/Game/Blueprint/Actors/Props/BP_Checkpoint.BP_Checkpoint_C|GetArrow (Variables|Default|GetCurrentCheckpoint)))))
    (:Is%20Not%20Valid
      (bind _returnvalue (Actor|GetActorOfClass "/Script/Engine.PlayerStart"))
      (Utilities|IsValid _returnvalue
        (:Is%20Valid
          (LocalVariables|SetTransformToSpawn (Transformation|GetActorTransform _returnvalue))))))
  (bind _returnvalue_2 (Game|SpawnActorfromClass "/Game/Blueprint/Core/P_MainChara.P_MainChara_C" (LocalVariables|GetTransformToSpawn) "Undefined" "MultiplyWithRoot" 0 0))
  (Pawn|Possess (Game|GetPlayerController 0) _returnvalue_2)
  (return))

(fn SetPause
  (params (isPause :type Boolean))
  (bind _hudparkourrace (Variables|Default|GetHudParkourRace))
  (bind _hudui (Variables|/Game/Blueprint/Core/HUD_ParkourRace.HUD_ParkourRace_C|GetHudUi _hudparkourrace))
  (Default|SetPause (Variables|Default|GetHudParkourRace) isPause)
  (Game|SetGamePaused isPause)
  (Default|PlayAnim _hudui (Variables|/Game/Blueprint/UI/W_HUDWidget.W_HUDWidget_C|GetPauseAnim _hudui) 1.0))

(fn OpenLevelName
  (params (Level :type Name))
  (Game|OpenLevel(byName) Level))